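; Dialogue component that runs data-table-driven conversations in a WB_dialogue widget, switching input mode and mouse cursor as it opens and closes.
; Interact opens or advances dialogue, with each row supplying text, next row and table, and end flag.
; Open-ended rows spawn Options1 choices only when the widget is created.
; optionselected shows the chosen row, then immediately closes if it ends or advances to the next.
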(event Custom|option%20selected
  (params (RowName :type Name) (DataTable :type Data%20Table%20Object%20Reference))
  (bind _returnvalue (Game|GetPlayerController 0))
  (bind _returnvalue_2 (Game|GetPlayerController 0))
  (bind _returnvalue_3 (Utilities|GetDataTableRow DataTable RowName)
    (:then
      (Widget|Panel|ClearChildren (Variables|/Game/Blueprints/dialogue/WB_dialogue.WB_dialogue_C|Getoptionscrollbox (Variables|Default|Getdialogue%20widget)))
      (Default|UpdateDialogue (Variables|Default|Getdialogue%20widget) (.Dialogue (Utilities|Struct|BreakBP_structure _returnvalue_3)))
      (Variables|Default|SetRow%20Name (.Row (Utilities|Struct|BreakBP_structure _returnvalue_3)))
      (Variables|Default|Setend%20dialogue (.enddialogue (Utilities|Struct|BreakBP_structure _returnvalue_3)))
      (Variables|Default|SetData%20Table (.DataTable (Utilities|Struct|BreakBP_structure _returnvalue_3)))
      (if (Variables|Default|Getend%20dialogue)
        (Widget|RemovefromParent (Variables|Default|Getdialogue%20widget))
        (Variables|Default|Setend%20dialogue false)
        (Variables|Default|Setdialogue%20widget 0)
        (Input|SetInputModeGameOnly _returnvalue_2 false)
        (Variables|/Script/Engine.PlayerController|SetbShowMouseCursor _returnvalue_2 false)
        (else
          (Utilities|IsValid (Variables|Default|Getdialogue%20widget)
            (:Is%20Valid
              (bind _returnvalue_4 (Utilities|GetDataTableRow (Variables|Default|GetData%20Table) (Variables|Default|GetRow%20Name))
                (:then
                  (Default|UpdateDialogue (Variables|Default|Getdialogue%20widget) (.Dialogue (Utilities|Struct|BreakBP_structure _returnvalue_4)))
                  (Variables|Default|SetRow%20Name (.Row (Utilities|Struct|BreakBP_structure _returnvalue_4)))
                  (Variables|Default|SetData%20Table (.DataTable (Utilities|Struct|BreakBP_structure _returnvalue_4)))
                  (Variables|Default|Setend%20dialogue (.enddialogue (Utilities|Struct|BreakBP_structure _returnvalue_4))))))
            (:Is%20Not%20Valid
              (bind _returnvalue_5 (Utilities|GetDataTableRow (Variables|Default|GetData%20Table) (Variables|Default|GetRow%20Name))
                (:then
                  (bind _returnvalue_6 (UserInterface|CreateWidget "/Game/Blueprints/dialogue/WB_dialogue.WB_dialogue_C" 0 (Utilities|Text|ToText(Name) (Variables|Default|GetName)) (.Dialogue (Utilities|Struct|BreakBP_structure _returnvalue_5))))
                  (bind _output_get (Variables|Default|Setdialogue%20widget _returnvalue_6))
                  (UserInterface|Viewport|AddtoViewport _output_get 0)
                  (Variables|Default|SetRow%20Name (.Row (Utilities|Struct|BreakBP_structure _returnvalue_5)))
                  (Variables|Default|SetData%20Table (.DataTable (Utilities|Struct|BreakBP_structure _returnvalue_5)))
                  (Variables|Default|Setend%20dialogue (.enddialogue (Utilities|Struct|BreakBP_structure _returnvalue_5)))
                  (Input|SetInputModeGameandUI _returnvalue 0 "DoNotLock" true false)
                  (Variables|/Script/Engine.PlayerController|SetbShowMouseCursor _returnvalue true)
                  (if (.openended? (Utilities|Struct|BreakBP_structure _returnvalue_5))
                    (for _array_element (.openendedoptions (Utilities|Struct|BreakBP_structure _returnvalue_5))
                      (bind _returnvalue_7 (UserInterface|CreateWidget "/Game/Blueprints/dialogue/options1.options1_C" 0 (Utilities|Text|ToText(Name) (.optionName (Utilities|Struct|BreakoptionsDaiolgue1 _array_element))) self (.row (Utilities|Struct|BreakoptionsDaiolgue1 _array_element)) (.datatable (Utilities|Struct|BreakoptionsDaiolgue1 _array_element))))
                      (Widget|Panel|AddChild (Variables|/Game/Blueprints/dialogue/WB_dialogue.WB_dialogue_C|Getoptionscrollbox (Variables|Default|Getdialogue%20widget)) _returnvalue_7))))))))))))

(event EventBeginPlay)

(event EventTick
  (params (DeltaSeconds :type Float%20%28single-precision%29)))

(event EventInteract
  (params (playerref :type BP%20Third%20Person%20Character%20Object%20Reference))
  (bind _returnvalue (Game|GetPlayerController 0))
  (bind _returnvalue_2 (Game|GetPlayerController 0))
  (if (Variables|Default|Getend%20dialogue)
    (Widget|RemovefromParent (Variables|Default|Getdialogue%20widget))
    (Variables|Default|Setend%20dialogue false)
    (Variables|Default|Setdialogue%20widget 0)
    (Input|SetInputModeGameOnly _returnvalue_2 false)
    (Variables|/Script/Engine.PlayerController|SetbShowMouseCursor _returnvalue_2 false)
    (else
      (Utilities|IsValid (Variables|Default|Getdialogue%20widget)
        (:Is%20Valid
          (bind _returnvalue_3 (Utilities|GetDataTableRow (Variables|Default|GetData%20Table) (Variables|Default|GetRow%20Name))
            (:then
              (Default|UpdateDialogue (Variables|Default|Getdialogue%20widget) (.Dialogue (Utilities|Struct|BreakBP_structure _returnvalue_3)))
              (Variables|Default|SetRow%20Name (.Row (Utilities|Struct|BreakBP_structure _returnvalue_3)))
              (Variables|Default|SetData%20Table (.DataTable (Utilities|Struct|BreakBP_structure _returnvalue_3)))
              (Variables|Default|Setend%20dialogue (.enddialogue (Utilities|Struct|BreakBP_structure _returnvalue_3))))))
        (:Is%20Not%20Valid
          (bind _returnvalue_4 (Utilities|GetDataTableRow (Variables|Default|GetData%20Table) (Variables|Default|GetRow%20Name))
            (:then
              (bind _returnvalue_5 (UserInterface|CreateWidget "/Game/Blueprints/dialogue/WB_dialogue.WB_dialogue_C" 0 (Utilities|Text|ToText(Name) (Variables|Default|GetName)) (.Dialogue (Utilities|Struct|BreakBP_structure _returnvalue_4))))
              (bind _output_get (Variables|Default|Setdialogue%20widget _returnvalue_5))
              (UserInterface|Viewport|AddtoViewport _output_get 0)
              (Variables|Default|SetRow%20Name (.Row (Utilities|Struct|BreakBP_structure _returnvalue_4)))
              (Variables|Default|SetData%20Table (.DataTable (Utilities|Struct|BreakBP_structure _returnvalue_4)))
              (Variables|Default|Setend%20dialogue (.enddialogue (Utilities|Struct|BreakBP_structure _returnvalue_4)))
              (Input|SetInputModeGameandUI _returnvalue 0 "DoNotLock" true false)
              (Variables|/Script/Engine.PlayerController|SetbShowMouseCursor _returnvalue true)
              (if (.openended? (Utilities|Struct|BreakBP_structure _returnvalue_4))
                (for _array_element (.openendedoptions (Utilities|Struct|BreakBP_structure _returnvalue_4))
                  (bind _returnvalue_6 (UserInterface|CreateWidget "/Game/Blueprints/dialogue/options1.options1_C" 0 (Utilities|Text|ToText(Name) (.optionName (Utilities|Struct|BreakoptionsDaiolgue1 _array_element))) self (.row (Utilities|Struct|BreakoptionsDaiolgue1 _array_element)) (.datatable (Utilities|Struct|BreakoptionsDaiolgue1 _array_element))))
                  (Widget|Panel|AddChild (Variables|/Game/Blueprints/dialogue/WB_dialogue.WB_dialogue_C|Getoptionscrollbox (Variables|Default|Getdialogue%20widget)) _returnvalue_6))))))))))

(event EventLeave
  (bind _returnvalue (Game|GetPlayerController 0))
  (Utilities|IsValid (Variables|Default|Getdialogue%20widget)
    (:Is%20Valid
      (Widget|RemovefromParent (Variables|Default|Getdialogue%20widget))
      (Variables|Default|Setend%20dialogue false)
      (Variables|Default|Setdialogue%20widget 0)
      (Input|SetInputModeGameOnly _returnvalue false)
      (Variables|/Script/Engine.PlayerController|SetbShowMouseCursor _returnvalue false))))
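; AI pawn that roams random reachable navmesh points and chases the player when it detects something, playing an explosion sound.
; Pawn sensing, perception updates and stimuli source activation all trigger the chase, with a retriggerable delay resuming roaming.
; Each tick, the game instance's Camo flag disables perception sight and shrinks pawn sensing radius, restoring both otherwise.
; The Chase function called on move failure is empty.
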(event OnTargetPerceptionUpdated(AIPerception)
  (params (Actor :type Actor%20Object%20Reference) (Stimulus :type AI%20Stimulus%20Structure))
  (Utilities|FlowControl|Sequence
    (:then_0
      (Audio|PlaySoundatLocation "/Game/StarterContent/Audio/Explosion01.Explosion01" "0, 0, 0" "0, 0, 0" 1.0 1.0 0.0 0 0 0 0)
      (AI|AIMoveTo self "0, 0, 0" (Game|GetPlayerCharacter 0) 1.0 false
        (:then
          (Utilities|FlowControl|Delay 0.3))
        (:OnFail
          (CallFunction|Chase))))
    (:then_1
      (Utilities|FlowControl|RetriggerableDelay 1.0)
      (CallFunction|RandomRoam))))

(event OnSeePawn(PawnSensing)
  (params (Pawn :type Pawn%20Object%20Reference))
  (Utilities|FlowControl|Sequence
    (:then_0
      (Audio|PlaySoundatLocation "/Game/StarterContent/Audio/Explosion01.Explosion01" "0, 0, 0" "0, 0, 0" 1.0 1.0 0.0 0 0 0 0)
      (AI|AIMoveTo self "0, 0, 0" (Game|GetPlayerCharacter 0) 1.0 false
        (:then
          (Utilities|FlowControl|Delay 0.3))
        (:OnFail
          (CallFunction|Chase))))
    (:then_1
      (Utilities|FlowControl|RetriggerableDelay 1.0)
      (CallFunction|RandomRoam))))

(event OnComponentActivated(AIPerceptionStimuliSource)
  (params (Component :type Actor%20Component%20Object%20Reference) (bReset :type Boolean))
  (Utilities|FlowControl|Sequence
    (:then_0
      (Audio|PlaySoundatLocation "/Game/StarterContent/Audio/Explosion01.Explosion01" "0, 0, 0" "0, 0, 0" 1.0 1.0 0.0 0 0 0 0)
      (AI|AIMoveTo self "0, 0, 0" (Game|GetPlayerCharacter 0) 1.0 false
        (:then
          (Utilities|FlowControl|Delay 0.3))
        (:OnFail
          (CallFunction|Chase))))
    (:then_1
      (Utilities|FlowControl|RetriggerableDelay 1.0)
      (CallFunction|RandomRoam))))

(event Custom|Random%20Roam
  (AI|AIMoveTo self (.RandomLocation (AI|Navigation|GetRandomReachablePointinRadius (Transformation|GetActorLocation) 5e+03 0 "/Script/AIModule.NavFilter_AIControllerDefault")) 0 1.0 false
    (:OnSuccess
      (CallFunction|RandomRoam))))

(event EventBeginPlay
  (AI|AIMoveTo self (.RandomLocation (AI|Navigation|GetRandomReachablePointinRadius (Transformation|GetActorLocation) 5e+03 0 "/Script/AIModule.NavFilter_AIControllerDefault")) 0 1.0 false
    (:OnSuccess
      (CallFunction|RandomRoam))))

(event Collision|EventActorBeginOverlap
  (params (OtherActor :type Actor%20Object%20Reference)))

(event EventTick
  (params (DeltaSeconds :type Float%20%28single-precision%29))
  (bind _asbp_game_instance_f (Utilities|Casting|CastTobp_GameInstanceF (Game|GetGameInstance)))
  (if (Variables|/Game/Blueprints/bp_GameInstanceF.bp_GameInstanceF_C|GetCamo? _asbp_game_instance_f)
    (Class|AIPerceptionComponent|SetSenseEnabled (Variables|Default|GetAIPerception) "/Script/AIModule.AISense_Sight" false)
    (Variables|/Script/AIModule.PawnSensingComponent|SetSightRadius (Variables|Default|GetPawnSensing) 5.0)
    (else
      (Class|AIPerceptionComponent|SetSenseEnabled (Variables|Default|GetAIPerception) "/Script/AIModule.AISense_Sight" true)
      (Variables|/Script/AIModule.PawnSensingComponent|SetSightRadius (Variables|Default|GetPawnSensing) 5e+03))))

(fn ConstructionScript)

(fn Chase)
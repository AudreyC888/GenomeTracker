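; Teleporter destination pad placed in the level, with a configurable name label, plate color and plate scale.
; The construction script applies those settings to the text and plate mesh, keeping the plate thin.
; It then finds every Teleporter_Sender targeting this destination and refreshes its name, color, rotation and scale, so linked senders stay in sync while editing.
; It has no active runtime logic.
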(event EventBeginPlay)

(event Collision|EventActorBeginOverlap
  (params (OtherActor :type Actor%20Object%20Reference)))

(event EventTick
  (params (DeltaSeconds :type Float%20%28single-precision%29)))

(fn ConstructionScript
  (CallFunction|UpdateName)
  (CallFunction|UpdateColor)
  (CallFunction|UpdateScale)
  (CallFunction|UpdateSenders))

(fn UpdateName
  (Rendering|Components|TextRender|SetText (Variables|Default|GetName) (Variables|Default|GetDestinationName)))

(fn UpdateColor
  (Rendering|Material|SetVectorParameterValueonMaterials (Variables|Default|GetPlate) "Base Color" (Math|Conversions|ToVector(LinearColor) (Variables|Default|GetColor))))

(fn UpdateScale
  (bind _platescale (Variables|Default|GetPlateScale))
  (Transformation|SetWorldScale3D (Variables|Default|GetPlate) (Math|Vector|MakeVector _platescale _platescale 0.02)))

(fn UpdateSenders
  (bind _outactors (Actor|GetAllActorsOfClass "/Game/Blueprints/Teleporter_Sender.Teleporter_Sender_C"))
  (for _array_element _outactors
    (if (== (Variables|/Game/Blueprints/Teleporter_Sender.Teleporter_Sender_C|GetDestination _array_element) self)
      (Default|UpdateName _array_element)
      (Default|UpdateColor _array_element)
      (Default|UpdateRotation _array_element)
      (Default|UpdateScale _array_element))))